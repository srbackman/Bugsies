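; First-person player character that commands bugs, picks up items and uses them on doors, and opens pause and win screens.
; Tick applies look and movement, pins the camera to head sockets, then runs the hand state machine.
; Forward box traces message targets, with UpdateHandControl setting state and type under a timed reset.
; Clicks select bugs or send them to targets or light-marked surface points.
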(event Input|EnhancedActionEvents|EnhancedInputActionIA_Move
  (params (ActionValue :type Vector%202D%20Structure) (ElapsedSeconds :type Float%20%28double-precision%29) (TriggeredSeconds :type Float%20%28double-precision%29) (InputAction :type Input%20Action%20Object%20Reference :default "/Game/Input/IA_Move.IA_Move"))
  (Variables|Default|SetMoveInput ActionValue))

(event Input|EnhancedActionEvents|EnhancedInputActionIA_Look
  (params (ActionValue :type Vector%202D%20Structure) (ElapsedSeconds :type Float%20%28double-precision%29) (TriggeredSeconds :type Float%20%28double-precision%29) (InputAction :type Input%20Action%20Object%20Reference :default "/Game/Input/IA_Look.IA_Look"))
  (Variables|Look|SetLookInput ActionValue))

(event Input|EnhancedActionEvents|EnhancedInputActionIA_Interact
  (params (ActionValue :type Boolean) (ElapsedSeconds :type Float%20%28double-precision%29) (TriggeredSeconds :type Float%20%28double-precision%29) (InputAction :type Input%20Action%20Object%20Reference :default "/Game/Input/IA_Interact.IA_Interact"))
  (Variables|Default|SetClickTriggered true))

(event Input|EnhancedActionEvents|EnhancedInputActionIA_ESC
  (params (ActionValue :type Boolean) (ElapsedSeconds :type Float%20%28double-precision%29) (TriggeredSeconds :type Float%20%28double-precision%29) (InputAction :type Input%20Action%20Object%20Reference :default "/Game/Input/IA_ESC.IA_ESC"))
  (bind _returnvalue (Game|GetPlayerController 0))
  (bind _returnvalue_2 (UserInterface|CreateWidget "/Game/Widget/WBP_PauseMenu.WBP_PauseMenu_C"))
  (UserInterface|Viewport|AddtoViewport _returnvalue_2 0)
  (Game|SetGamePaused true)
  (Variables|/Script/Engine.PlayerController|SetbShowMouseCursor _returnvalue true)
  (Input|SetInputModeUIOnly _returnvalue _returnvalue_2 "LockAlways" false))

(event Input|EnhancedActionEvents|EnhancedInputActionIA_Deselect
  (params (ActionValue :type Boolean) (ElapsedSeconds :type Float%20%28double-precision%29) (TriggeredSeconds :type Float%20%28double-precision%29) (InputAction :type Input%20Action%20Object%20Reference :default "/Game/Input/IA_Deselect.IA_Deselect"))
  (bind _currentinteract (Variables|Default|GetCurrentInteract))
  (Utilities|IsValid _currentinteract
    (:Is%20Valid
      (Class|BPIPlayerInteract|Interact(Message) _currentinteract true)
      (CallFunction|ResetSelection)
      (Rendering|Components|Light|SetIntensity (Variables|Default|GetDestinationLight) 0.0))))

(event EventBeginPlay
  ;[1 1 1] InputMapping
  (bind _asplayer_controller (Utilities|Casting|CastToPlayerController (Pawn|GetController)))
  (Input|AddMappingContext (PlayerController|LocalPlayerSubsystems|GetEnhancedInputLocalPlayerSubsystem _asplayer_controller) (Variables|Default|GetInputMapping) 0 "(bIgnoreAllPressedKeysUntilRelease=True,bForceImmediately=False,bNotifyUserSettings=False)"))

(event EventTick
  (params (DeltaSeconds :type Float%20%28single-precision%29))
  (Utilities|FlowControl|Sequence
    (:then_0
      ;[1 1 1] Movement
      (CallFunction|UpdateZRotation DeltaSeconds)
      (CallFunction|UpdateCameraLocationRotation)
      (CallFunction|UpdateMove))
    (:then_1
      (CallFunction|HandControl))))

(fn ConstructionScript)

(fn UpdateCameraLocationRotation
  (bind _head (Variables|Default|GetHead))
  (bind _returnvalue (Transformation|GetSocketLocation _head "Eye2"))
  (Transformation|SetWorldLocationAndRotation (Variables|Default|GetCamera) _returnvalue (Math|Rotator|MakeRotfromX (- _returnvalue (Transformation|GetSocketLocation _head "Eye1"))) false false))

(fn UpdateZRotation
  (params (DeltaSeconds :type Float%20%28double-precision%29))
  (bind _lookspeed (Variables|Look|GetLookSpeed))
  (Variables|Look|SetLookUpDown (Math|Float|Clamp(Float) (+ (Variables|Look|GetLookUpDown) (* (* (.Y (Math|Vector2D|BreakVector2D (Variables|Look|GetLookInput))) DeltaSeconds) (* _lookspeed 0.01)))))
  (Transformation|SetActorRotation (Math|Rotator|CombineRotators (Transformation|GetActorRotation) (Math|Rotator|MakeRotator 0.0 0.0 (* (* (.X (Math|Vector2D|BreakVector2D (Variables|Look|GetLookInput))) DeltaSeconds) _lookspeed))))
  (Variables|Look|SetLookInput ""))

(fn UpdateMove
  (Pawn|Input|AddMovementInput (Math|Vector|RotateVector (Math|Vector|MakeVector (.X (Math|Vector2D|BreakVector2D (Variables|Default|GetMoveInput))) (.Y (Math|Vector2D|BreakVector2D (Variables|Default|GetMoveInput))) 0.0) (Transformation|GetActorRotation)) 1.0 false)
  (Variables|Default|SetMoveInput ""))

(fn SquareTraceForward
  (bind _camera (Variables|Default|GetCamera))
  (bind _interactchecksize (Variables|Default|GetInteractCheckSize))
  (bind _returnvalue (Transformation|GetWorldLocation _camera))
  (bind (_outhit _returnvalue_2) (Class|KismetSystemLibrary|BoxTraceSingleforObjects _returnvalue (+ _returnvalue (* (Math|Vector|GetForwardVector _camera) (Variables|Default|GetCommandRange))) (Math|Vector|MakeVector _interactchecksize _interactchecksize _interactchecksize) (Transformation|GetWorldRotation _camera) (Utilities|Array|MakeArray "ObjectTypeQuery3" "ObjectTypeQuery2" "ObjectTypeQuery4") false 0 "None" true))
  (if _returnvalue_2
    (return (.HitActor (Collision|BreakHitResult _outhit)))
    (else
      (return 0))))

(fn HandControl
  (bind _destinationlight (Variables|Default|GetDestinationLight))
  (bind _interactionth (Variables|Default|GetInteractionTH))
  (bind _camera (Variables|Default|GetCamera))
  (bind _returnvalue (Transformation|GetWorldLocation _camera))
  (switch Utilities|FlowControl|Switch|SwitchonE_HandState (Variables|Default|GetHandState)
    (:NewEnumerator0
      (bind _foundactor (CallFunction|SquareTraceForward :!label _label))
      (Utilities|IsValid _foundactor
        (:Is%20Valid
          (switch Utilities|FlowControl|Switch|SwitchonE_ActorType (Variables|Default|GetActorType)
            (:NewEnumerator0
              (Class|BPIPlayerInteract|IsValidTarget(Message) _foundactor self :!label _label_2) ; HighlightBugOrItem
              (Rendering|Components|Light|SetIntensity (Variables|Default|GetDestinationLight) 0.0)
              (Variables|Default|SetClickTriggered false))
            (:NewEnumerator1
              (if (Variables|Default|GetClickTriggered) ; Click
                (Variables|Default|SetClickTriggered false)
                (Utilities|IsValid (Variables|Default|GetCurrentInteract)
                  (:Is%20Valid
                    (if (== (Variables|Default|GetCurrentInteract) _foundactor)
                      ;[1 1 1] UnSelect
                      (Class|BPIPlayerInteract|Interact(Message) _foundactor true)
                      (CallFunction|ResetSelection)
                      (else
                        ;[1 1 1] SetDestinationToAnotherBugOrItem
                        (Class|BPIPlayerInteract|SetDestination(Message) (Variables|Default|GetCurrentInteract) (Transformation|GetActorLocation _foundactor) true)
                        (CallFunction|ResetSelection))))
                  (:Is%20Not%20Valid
                    ;[1 1 1] BasicInteract
                    (Class|BPIPlayerInteract|Interact(Message) _foundactor false)
                    (Variables|Default|SetCurrentInteract _foundactor)
                    (if (Utilities|Time|IsTimerActivebyHandle _interactionth)
                      (Utilities|Time|ClearandInvalidateTimerbyHandle _interactionth))))
                (elif (!= _foundactor (Variables|Default|GetCurrentInteract))
                  (goto _label_2))))
            (:NewEnumerator2
              ;[1 1 1] Item
              (if (>= (Variables|Default|GetPickUpRange) (Math|Vector|Distance(Vector) (Transformation|GetActorLocation self) (Transformation|GetActorLocation _foundactor)))
                (Variables|Default|SetHandState "NewEnumerator2")
                (if (Variables|Default|GetClickTriggered) ; Click
                  (Variables|Default|SetClickTriggered false)
                  (Class|BPIPlayerInteract|Interact(Message) _foundactor false)
                  (Variables|Default|SetCurrentInteract _foundactor)
                  (else
                    (goto _label_2)))
                (else
                  (Variables|Default|SetHandState "NewEnumerator1")
                  (Variables|Default|SetClickTriggered false)
                  (goto _label_2))))))
        (:Is%20Not%20Valid
          ;[1 1 1] MoveBugToLocation
          (bind (_outhit _returnvalue_2) (Collision|LineTraceForObjects _returnvalue (+ _returnvalue (* (Math|Vector|GetForwardVector _camera) (Variables|Default|GetCommandRange))) (Utilities|Array|MakeArray "ObjectTypeQuery1") false 0 "None"))
          (if _returnvalue_2
            (if (Variables|Default|GetClickTriggered) ; Click
              (Variables|Default|SetClickTriggered false)
              (Class|BPIPlayerInteract|SetDestination(Message) (Variables|Default|GetCurrentInteract) (.ImpactPoint (Collision|BreakHitResult _outhit)) false)
              (Rendering|Components|Light|SetIntensity _destinationlight 0.0)
              (else
                (Transformation|SetWorldLocation _destinationlight (+ (.ImpactPoint (Collision|BreakHitResult _outhit)) (* (.ImpactNormal (Collision|BreakHitResult _outhit)) (Variables|Default|GetIndicatorElevation))) false false)
                (Rendering|Components|Light|SetIntensity _destinationlight 2e+01)))
            (else
              (Rendering|Components|Light|SetIntensity _destinationlight 0.0)
              (Variables|Default|SetClickTriggered false))))))
    (:NewEnumerator1
      (goto _label))
    (:NewEnumerator2
      (goto _label))
    (:NewEnumerator3
      (CallFunction|HandinUse))))

(fn UpdateHandControl
  (params (NewState :type E_HandState%20Enum :default "NewEnumerator0") (Type :type E_ActorType%20Enum :default "NewEnumerator0"))
  (if (not (and (Utilities|Enum|Equal(Enum) Type "NewEnumerator3") (Utilities|Enum|Equal(Enum) (Variables|Default|GetActorType) "NewEnumerator1")))
    (Variables|Default|SetHandState NewState)
    (Variables|Default|SetActorType Type)
    (bind _returnvalue (Utilities|Time|SetTimerbyFunctionName 0 "ResetPointingState" 0.3))
    (Variables|Default|SetInteractionTH _returnvalue)))

(fn ResetPointingState
  (if (Utilities|Enum|Equal(Enum) (Variables|Default|GetActorType) "NewEnumerator3")
    (CallFunction|ResetSelection)
    (elif (Utilities|Enum|NotEqual(Enum) (Variables|Default|GetHandState) "NewEnumerator3")
      (Variables|Default|SetHandState "NewEnumerator0"))))

(fn ResetSelection
  (Variables|Default|SetCurrentInteract 0)
  (Variables|Default|SetHandState "NewEnumerator0")
  (Variables|Default|SetActorType "NewEnumerator0"))

(fn IsHandFree
  (return (not (Utilities|IsValid (Variables|Default|GetCurrentInteract)))))

(fn GetHandSlotLocRot
  (bind _mesh (Variables|Character|GetMesh))
  (bind _returnvalue (Transformation|GetSocketLocation _mesh "Grab2"))
  (return _returnvalue (Math|Rotator|CombineRotators (Math|Rotator|MakeRotationfromAxes (Math|Vector|Normalize (- (Transformation|GetSocketLocation _mesh "Grab1") _returnvalue)) (Math|Vector|GetRightVector _mesh) "0, 0, 0") "0, 0, 0")))

(fn HandinUse
  (switch Utilities|FlowControl|Switch|SwitchonE_ActorType (Variables|Default|GetActorType)
    (:NewEnumerator2
      (bind _foundactor (CallFunction|SquareTraceForward)) ; Door
      (Utilities|IsValid _foundactor
        (:Is%20Valid
          (Class|BPIPlayerInteract|IsValidTarget(Message) _foundactor self)
          (if (Utilities|Enum|Equal(Enum) (Variables|Default|GetActorType) "NewEnumerator3")
            (if (Variables|Default|GetClickTriggered) ; Click
              (Variables|Default|SetClickTriggered false)
              (Class|BPIPlayerInteract|Interact(Message) _foundactor false) ; Door
              (Class|BPIPlayerInteract|Interact(Message) (Variables|Default|GetCurrentInteract) false) ; Key
              (CallFunction|ResetSelection)
              (else
                (CallFunction|UpdateHandControl "NewEnumerator3" "NewEnumerator2" :!label _label)
                (Variables|Default|SetClickTriggered false)))
            (else
              (goto _label))))
        (:Is%20Not%20Valid
          (goto _label))))))

(fn WinScreen
  (bind _returnvalue (Game|GetPlayerController 0))
  (Game|SetGamePaused true)
  (bind _returnvalue_2 (UserInterface|CreateWidget "/Game/Widget/WBP_WinScreen.WBP_WinScreen_C"))
  (UserInterface|Viewport|AddtoViewport _returnvalue_2 0)
  (Variables|/Script/Engine.PlayerController|SetbShowMouseCursor _returnvalue true)
  (Input|SetInputModeUIOnly _returnvalue _returnvalue_2 "LockAlways" false))

(fn Interact
  (params (UnSelect :type Boolean)))

(fn IsValidTarget
  (params (Player :type BP%20Player%20Object%20Reference))
  (return))