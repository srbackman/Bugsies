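; Interactable door that opens once targeted and used by the player, with no logic to close it again.
; While closed, being targeted updates the player's hand control based on whether a hand is free and lights up a highlight.
; A timer by function name switches the highlight off after a set delay.
; Interacting snaps the hinge a quarter turn without animation, marks the door open and plays audio.
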(event EventBeginPlay)

(event Collision|EventActorBeginOverlap
  (params (OtherActor :type Actor%20Object%20Reference)))

(event EventTick
  (params (DeltaSeconds :type Float%20%28single-precision%29)))

(event EventInteract
  (params (UnSelect :type Boolean))
  (CallFunction|Open))

(event EventIsValidTarget
  (params (Player :type BP%20Player%20Object%20Reference))
  (if (not (Variables|Default|GetIsOpen))
    (bind _result (Default|IsHandFree Player))
    (if _result
      (Default|UpdateHandControl Player "NewEnumerator1" "NewEnumerator0")
      (else
        (Default|UpdateHandControl Player "NewEnumerator3" "NewEnumerator3")))
    (Rendering|Components|Light|SetIntensity (Variables|Default|GetHighlight) (Variables|Default|GetHighlightBrightness))
    (bind _returnvalue (Utilities|Time|SetTimerbyFunctionName 0 "ResetHighlight" (Variables|Default|GetHighlightResetTime)))
    (Variables|Default|SetHighlightTH _returnvalue)))

(fn ConstructionScript)

(fn ResetHighlight
  (Rendering|Components|Light|SetIntensity (Variables|Default|GetHighlight) 0.0))

(fn Open
  (Transformation|SetRelativeRotation (Variables|Default|GetHinge) "0.000000,90.000000,0.000000" false false)
  (Variables|Default|SetIsOpen true)
  (Audio|Components|Audio|Play (Variables|Default|GetAudio) 0.0))