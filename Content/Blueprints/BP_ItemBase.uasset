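; Base item actor that the player can highlight, pick up, drop, push or use on a door.
; A state variable drives it: targeting lights a timed highlight and updates the player's hand control, while Interact toggles gravity and collision type.
; Held items follow the player's hand slot each Tick rather than attaching; items used on doors are hidden and moved below the world.
; Push applies an outward-and-upward impulse, and mesh hits play audio.
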(event OnComponentHit(StaticMesh)
  (params (HitComponent :type Primitive%20Component%20Object%20Reference) (OtherActor :type Actor%20Object%20Reference) (OtherComp :type Primitive%20Component%20Object%20Reference) (NormalImpulse :type Vector :default "0, 0, 0") (Hit :type Hit%20Result%20Structure%20%28by%20ref%29))
  (Audio|Components|Audio|Play (Variables|Default|GetAudio) 0.0))

(event Custom|OnActorHit_Event
  (params (SelfActor :type Actor%20Object%20Reference) (OtherActor :type Actor%20Object%20Reference) (NormalImpulse :type Vector) (Hit :type Hit%20Result%20Structure%20%28by%20ref%29)))

(event EventBeginPlay
  (EventDispatchers|BindEventtoOnActorHit (delegate Custom|OnActorHit_Event)))

(event EventIsValidTarget
  (params (Player :type BP%20Player%20Object%20Reference))
  ;[1 1 1] IsValidTarget
  (Utilities|IsValid (Variables|Default|GetPlayer)
    (:Is%20Valid
      (switch Utilities|FlowControl|Switch|SwitchonE_ItemState (Variables|Default|GetState)
        (:NewEnumerator0
          (bind _result (Default|IsHandFree Player))
          (if _result
            (if (Utilities|Enum|Equal(Enum) (Variables|/Game/Blueprints/BP_Player.BP_Player_C|GetHandState Player) "NewEnumerator2")
              _
              (else
                (Default|UpdateHandControl Player "NewEnumerator1" "NewEnumerator2"))))
          (Rendering|Components|Light|SetIntensity (Variables|Default|GetHighlight) (Variables|Default|GetHighlightBrightness))
          (bind _returnvalue (Utilities|Time|SetTimerbyFunctionName 0 "ResetHighlight" (Variables|Default|GetHighlightResetTime)))
          (Variables|Default|SetHighlightTH _returnvalue))))
    (:Is%20Not%20Valid
      (Variables|Default|SetPlayer Player))))

(event EventTick
  (params (DeltaSeconds :type Float%20%28single-precision%29))
  ;[1 1 1] Tick
  (if (Utilities|Enum|Equal(Enum) (Variables|Default|GetState) "NewEnumerator1")
    (CallFunction|UpdateinHandLocation)))

(event EventPush
  (params (Actor :type Actor%20Object%20Reference) (Force :type Float%20%28double-precision%29))
  ;[1 1 1] Push
  (Physics|AddImpulse (Variables|Default|GetStaticMesh) (+ (* (Math|Vector|Normalize (- (Transformation|GetActorLocation self) (Transformation|GetActorLocation Actor))) Force) (* "0.000000,0.000000,1.000000" Force)) "None" true))

(event EventInteract
  (params (UnSelect :type Boolean))
  (bind _player (Variables|Default|GetPlayer))
  (bind _player_2 (Variables|Default|GetPlayer))
  (bind _staticmesh (Variables|Default|GetStaticMesh))
  ;[1 1 1] Interact
  (Utilities|IsValid _player
    (:Is%20Valid
      (if UnSelect
        (Variables|Default|SetState "NewEnumerator0") ; Drop
        (Default|UpdateHandControl _player_2 "NewEnumerator0" "NewEnumerator0")
        (Physics|SetEnableGravity _staticmesh true)
        (Collision|SetCollisionObjectType _staticmesh "ECC_PhysicsBody")
        (else
          (switch Utilities|FlowControl|Switch|SwitchonE_ActorType (Variables|/Game/Blueprints/BP_Player.BP_Player_C|GetActorType _player)
            (:NewEnumerator2
              (Variables|Default|SetState "NewEnumerator1") ; PickUp
              (Default|UpdateHandControl _player_2 "NewEnumerator3" "NewEnumerator2")
              (Physics|SetEnableGravity _staticmesh false)
              (Collision|SetCollisionObjectType _staticmesh "ECC_WorldStatic"))
            (:NewEnumerator3
              (Variables|Default|SetState "NewEnumerator2") ; UseOnDoor
              (Default|UpdateHandControl _player_2 "NewEnumerator0" "NewEnumerator0")
              (Rendering|SetActorHiddenInGame true)
              (Transformation|SetActorLocation "0.000000,0.000000,-1000.000000" false false))))))))

(fn ConstructionScript)

(fn ResetHighlight
  (Rendering|Components|Light|SetIntensity (Variables|Default|GetHighlight) 0.0))

(fn UpdateinHandLocation
  (bind (_location _rotation) (Default|GetHandSlotLocRot (Variables|Default|GetPlayer)))
  (Transformation|SetActorLocationAndRotation _location _rotation))